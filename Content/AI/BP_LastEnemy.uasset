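; BP_LastEnemy is an enemy AI pawn that chases the player once it spots them.
; Its PawnSensing component checks that the seen pawn is BP_Player, sets a SeePlayer flag and calls FollowPlayer.
; FollowPlayer issues a single AI MoveTo toward the player character when that flag is set, with debug prints along the way.
; The flag is never cleared here, and Tick is unused.
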(event OnSeePawn(PawnSensing)
  (params (Pawn :type Pawn%20Object%20Reference))
  (Utilities|Casting|CastToBP_Player Pawn)
  (Development|PrintString "Hello")
  (Variables|Default|SetbSeePlayer true)
  (CallFunction|FollowPlayer))

(event Custom|FollowPlayer
  (if (Variables|Default|GetbSeePlayer)
    (Development|PrintString "havetomove")
    (AI|AIMoveTo self "0, 0, 0" (Game|GetPlayerCharacter 0) 5.0 false)))

(event EventBeginPlay)

(event Collision|EventActorBeginOverlap
  (params (OtherActor :type Actor%20Object%20Reference)))

(event EventTick
  (params (DeltaSeconds :type Float%20%28single-precision%29)))

(fn ConstructionScript)