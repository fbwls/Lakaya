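; BP_AI is an AI actor that alternates between two patrol points, TP1 and TP2, and carries an AR4 weapon.
; Overlapping either point switches CurTP to the other and writes it to the TargetPoint blackboard key, which is also set on BeginPlay.
; A separate Patrol function repeats that blackboard write but is not called here.
; The construction script attaches AR4 to the mesh's WeaponSocket.
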(event EventBeginPlay
  (AI|Components|Blackboard|SetValueasObject (AI|GetBlackboard self) (Utilities|Name|MakeLiteralName "TargetPoint") (Variables|Default|GetCurTP)))

(event Collision|EventActorBeginOverlap
  (params (OtherActor :type Actor%20Object%20Reference))
  (if (== OtherActor (Variables|Default|GetTP1))
    (Variables|Default|SetCurTP (Variables|Default|GetTP2))
    (AI|Components|Blackboard|SetValueasObject (AI|GetBlackboard self) (Utilities|Name|MakeLiteralName "TargetPoint") (Variables|Default|GetCurTP) :!label _label)
    (elif (== OtherActor (Variables|Default|GetTP2))
      (Variables|Default|SetCurTP (Variables|Default|GetTP1))
      (goto _label))))

(fn ConstructionScript
  (Transformation|AttachComponentToComponent (Variables|Default|GetAR4) (Variables|Character|GetMesh) "WeaponSocket" "KeepWorld" "KeepWorld" "SnapToTarget" true))

(fn Patrol
  (AI|Components|Blackboard|SetValueasObject (AI|GetBlackboard self) (Utilities|Name|MakeLiteralName "TargetPoint") (Variables|Default|GetCurTP)))